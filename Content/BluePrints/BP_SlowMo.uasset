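; BP_SlowMo is a trigger volume that creates a slow-motion moment when the main character overlaps its box.
; The overlap plays a glass-breaking sound, spawns a RadialBurst effect, lowers the target GameSpeed and starts the SlowMoSpeed timeline.
; Timeline updates lerp global time dilation from its current value toward GameSpeed using the speed track.
; After a short Delay, GameSpeed returns to normal without restarting the timeline.
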(event OnComponentBeginOverlap(Box)
  (params (OverlappedComponent :type Primitive%20Component%20Object%20Reference) (OtherActor :type Actor%20Object%20Reference) (OtherComp :type Primitive%20Component%20Object%20Reference) (OtherBodyIndex :type Integer) (bFromSweep :type Boolean) (SweepResult :type Hit%20Result%20Structure%20%28by%20ref%29))
  (Utilities|Casting|CastToBP_MainCharacter OtherActor)
  (Audio|PlaySound2D "/Game/SFX/C_GlassBrokenSlowMo.C_GlassBrokenSlowMo" 1.0 1.0 0.0 0 0)
  (Variables|Default|SetGameSpeed 0.2)
  (Components|Timeline|PlayfromStart (Variables|Default|GetSlowMoSpeed))
  (Niagara|SpawnSystemAttached "/Niagara/DefaultAssets/Templates/Systems/RadialBurst.RadialBurst" (Variables|Default|GetDefaultSceneRoot) "None" "0,-50.000000,-10.000000" "0, 0, 0" "KeepRelativeOffset" false)
  (Utilities|FlowControl|Delay 1.5)
  (Variables|Default|SetGameSpeed 1.0))

(fn ConstructionScript)